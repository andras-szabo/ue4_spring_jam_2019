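; BP_Groove is an actor whose mesh the player rotates through input relayed by BP_PlayerController.
; On BeginPlay it binds to the controller's OnRotation dispatcher and responds only while IsActive is set.
; Each event adds the direction times RotationSpeed to the mesh's world roll, forcing pitch and yaw to zero, with no delta-time scaling.
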(event `self.ReceiveBeginPlay`
  (bind _asbp_player_controller (cast `/Game/Blueprints/BP_PlayerController` (`GameplayStatics.GetPlayerController` 0)))
  (add `/Game/Blueprints/BP_PlayerController.OnRotation` _asbp_player_controller (delegate `HandleRotation`)))

(event `HandleRotation`
  (params (Direction :type "Float (double-precision)"))
  (if (`self.IsActive`)
    (`self.Rotate` Direction)))

(fn `Rotate`
  (params (RotationSign :type "Float (double-precision)"))
  (`SceneComponent.K2_SetWorldRotation` (`self.Mesh`) (`KismetMathLibrary.MakeRotator` (+ (* RotationSign (`self.RotationSpeed`)) (.roll (`SceneComponent.K2_GetComponentRotation` (`self.Mesh`))))) false false))

(fn `UserConstructionScript`)