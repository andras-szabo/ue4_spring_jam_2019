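; BP_InGameSwitch is an overlap-triggered switch actor that broadcasts its on/off state through the OnSwitchStateChanged event dispatcher.
; Each begin overlap flips IsOn, fires the dispatcher with the new value and prints a debug "Hello".
; When IsToggleSwitch is false, end overlap flips and broadcasts again, giving momentary behavior.
; Overlaps are not filtered or counted, so multiple overlapping actors each flip the state.
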(event `self.ReceiveActorBeginOverlap`
  (params (OtherActor :type "Actor Object Reference"))
  ;[1 1 1] OnActorBeginOverlap => OnSwitchStateChanged
  (bind _output_get (set `self.IsOn` (not (`self.IsOn`))))
  (`self.OnSwitchStateChanged` _output_get)
  (`KismetSystemLibrary.PrintString` "Hello"))

(event `self.ReceiveActorEndOverlap`
  (params (OtherActor :type "Actor Object Reference"))
  ;[1 1 1] If not a simple toggle, then also call on end overlap
  (if (not (`self.IsToggleSwitch`))
    (bind _output_get (set `self.IsOn` (not (`self.IsOn`))))
    (`self.OnSwitchStateChanged` _output_get)))

(fn `UserConstructionScript`)