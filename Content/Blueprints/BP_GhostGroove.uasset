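; BP_GhostGroove is a groove that switches between a solid state and a non-colliding ghost state.
; SetGhostState swaps the mesh material and collision, and the construction script applies it from IsSolid.
; The player controller's ghost toggle event flips the state.
; Bound switch events recheck ActivatingSwitches, making the groove solid only when all are on, with leftover debug prints along that path.
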(event `self.ReceiveBeginPlay`
  (`parent.ReceiveBeginPlay`)
  (bind _asbp_player_controller (cast `/Game/Blueprints/BP_PlayerController` (`GameplayStatics.GetPlayerController` 0)))
  (add `/Game/Blueprints/BP_PlayerController.OnGhostToggle` _asbp_player_controller (delegate `HandleGhostToggle`))
  (for _array_element (`self.ActivatingSwitches`)
    (add `/Game/Blueprints/BP_InGameSwitch.OnSwitchStateChanged` _array_element (delegate `HandleSwitchStateChanged`))
    (`KismetSystemLibrary.PrintString` "bound")))

(event `HandleGhostToggle`
  (`self.SetGhostState` (not (`self.IsSolid`))))

(event `HandleSwitchStateChanged`
  (params (IsSwitchOn :type Boolean))
  (`KismetSystemLibrary.PrintString` "FFS" true true (struct :`G` 0.66 :`B` 1.0 :`A` 1.0) 8.0)
  (`self.HandleSwitchStateChange` IsSwitchOn))

(fn `HandleSwitchStateChange`
  (params (IsOn :type Boolean))
  (locals (AllSwitchesOn :type Boolean))
  (`KismetSystemLibrary.PrintString` "lolololo" true true (struct :`G` 0.66 :`B` 1.0 :`A` 1.0) 5.0)
  ;[1 1 1] If all activiating switches are on, then the groove is solid; otherwise it's a ghost.
  (set `local.AllSwitchesOn` true)
  (for _array_element (`self.ActivatingSwitches`)
    (if (not (`/Game/Blueprints/BP_InGameSwitch.IsOn` _array_element))
      (set `local.AllSwitchesOn` false)))
  (`self.SetGhostState` (`local.AllSwitchesOn`)))

(fn `SetGhostState`
  (params (IsSolid :type Boolean))
  (locals (CollisionEnabled :type "ECollisionEnabled Enum" :default "NoCollision"))
  ;[1 1 1] Set material and collision settings when changing ghost state
  (bind _output_get (set `self.IsSolid` IsSolid))
  (`PrimitiveComponent.SetMaterial` (`self.Mesh`) 0 (select `bool` _output_get :`false` (`self.GhostMaterial`) :`true` (`self.NormalMaterial`)))
  (if (`self.IsSolid`)
    (set `local.CollisionEnabled` "QueryAndPhysics")
    (else
      (set `local.CollisionEnabled` "NoCollision")))
  (`PrimitiveComponent.SetCollisionEnabled` (`self.Mesh`) (`local.CollisionEnabled`)))

(fn `UserConstructionScript`
  (locals (NewLocalVar_0 :type "/DatasmithContent/Blueprints/FBXImporter/BP_Switch Object Reference"))
  (`parent.UserConstructionScript`)
  (`self.SetGhostState` (`self.IsSolid`)))