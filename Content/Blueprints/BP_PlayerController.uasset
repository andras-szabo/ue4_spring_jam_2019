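; BP_PlayerController is a player controller that turns keyboard input into rotation and gravity-flip events.
; G and H hold left and right rotation flags, and Tick calls OnRotation with a signed direction each frame that exactly one is held.
; Space bar toggles the gravity-flipped state and immediately calls OnGravityFlip with the new value.
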(event `Key|H`
  (params (Key :type "Key Structure"))
  ;[1 1 1] Handle input
  (:`Pressed`
    (set `self.IsRotatingRight` true))
  (:`Released`
    (set `self.IsRotatingRight` false)))

(event `Key|SpaceBar`
  (params (Key :type "Key Structure"))
  ;[1 1 1] Handle input
  (:`Pressed`
    (bind _output_get (set `self.IsGravityFlipped` (not (`self.IsGravityFlipped`))))
    (`self.OnGravityFlip` _output_get)))

(event `Key|G`
  (params (Key :type "Key Structure"))
  ;[1 1 1] Handle input
  (:`Pressed`
    (set `self.IsRotatingLeft` true))
  (:`Released`
    (set `self.IsRotatingLeft` false)))

(event `self.ReceiveTick`
  (params (DeltaSeconds :type "Float (single-precision)"))
  ;[1 1 1] Send OnRotation calls on tick
  (if (!= (`self.IsRotatingRight`) (`self.IsRotatingLeft`))
    (if (`self.IsRotatingRight`)
      (set `self.RotationDirection` 1.0)
      (else
        (bind _output_get (set `self.RotationDirection` -1.0))))
    (`self.OnRotation` _output_get)))

(fn `UserConstructionScript`)