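; BP_WindVolume is a box volume that pushes physics-simulated static meshes inside it along a wind direction.
; Begin and end overlap events update a debug-printed counter and rebuild the mesh array with a box overlap query for PhysicsBody components.
; While the counter is above zero, Tick applies a slightly randomized, mass-independent acceleration force to each cached mesh.
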(event `self.Box.OnComponentBeginOverlap`
  (params (OverlappedComponent :type "PrimitiveComponent Object Reference") (OtherActor :type "Actor Object Reference") (OtherComp :type "PrimitiveComponent Object Reference") (OtherBodyIndex :type Integer) (bFromSweep :type Boolean) (SweepResult :type "HitResult Structure (by ref)"))
  ;[1 1 1] On begin and end overlap, refresh array of overlapping static mesh components
  (bind _result (`/Engine/EditorBlueprintResources/StandardMacros.IncrementInt` (`self.OverlappingActorCount`))
    (:`  `
      (`KismetSystemLibrary.PrintString` (`KismetStringLibrary.Conv_IntToString` _result))
      (`self.FindOverlappingStaticMeshComponents` :!label _label))))

(event `self.Box.OnComponentEndOverlap`
  (params (OverlappedComponent :type "PrimitiveComponent Object Reference") (OtherActor :type "Actor Object Reference") (OtherComp :type "PrimitiveComponent Object Reference") (OtherBodyIndex :type Integer))
  ;[1 1 1] On begin and end overlap, refresh array of overlapping static mesh components
  (bind _result (`/Engine/EditorBlueprintResources/StandardMacros.DecrementInt` (`self.OverlappingActorCount`))
    (:`  `
      (`KismetSystemLibrary.PrintString` (`KismetStringLibrary.Conv_IntToString` _result) true true (struct :`R` 1.0 :`G` 0.240154 :`B` 0.958786 :`A` 1.0))
      (goto _label))))

(event `self.ReceiveTick`
  (params (DeltaSeconds :type "Float (single-precision)"))
  ;[1 1 1] On tick, apply force to overlapping static mesh components
  (if (> (`self.OverlappingActorCount`) 0)
    (for _array_element (`self.OverlappingStaticMeshes`)
      (`PrimitiveComponent.AddForce` _array_element (* (`self.WindDirection`) (`KismetMathLibrary.RandomFloatInRange` 0.8 1.2)) "None" true))))

(fn `FindOverlappingStaticMeshComponents`
  (`KismetArrayLibrary.Array_Clear` (`self.OverlappingStaticMeshes`))
  (bind _outcomponents (`KismetSystemLibrary.BoxOverlapComponents` (`self.K2_GetActorLocation`) (`BoxComponent.GetScaledBoxExtent` (`self.Box`)) (`|MakeArray` "ObjectTypeQuery4" :!type "EObjectTypeQuery Enum") "/Script/Engine.StaticMeshComponent"))
  (for _array_element _outcomponents
    (bind _asstatic_mesh_component (cast `StaticMeshComponent` _array_element))
    (`KismetArrayLibrary.Array_Add` (`self.OverlappingStaticMeshes`) _asstatic_mesh_component)))

(fn `UserConstructionScript`)